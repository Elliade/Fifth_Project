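; BP_HitBox_First is a hit box actor that shrinks each time another actor stops overlapping it.
; BeginPlay caches five percent of the starting scale, and each end overlap subtracts that fixed step, so shrinkage is linear with no lower clamp.
; The new scale is printed for debugging, while begin overlap and the construction script only call their parent versions.
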(event EventBeginPlay
  (Variables|Default|SetOur%205%25 (* (Transformation|GetActorScale3D) 0.05)))

(event Collision|EventActorBeginOverlap
  (params (OtherActor :type Actor%20Object%20Reference))
  (|CallParentFunction OtherActor))

(event Collision|EventActorEndOverlap
  (params (OtherActor :type Actor%20Object%20Reference))
  (Transformation|SetActorScale3D (- (Transformation|GetActorScale3D) (Variables|Default|GetOur%205%25)))
  (Development|PrintString (Utilities|String|ToString(Vector) (Transformation|GetActorScale3D))))

(fn ConstructionScript
  (|CallParentFunction))