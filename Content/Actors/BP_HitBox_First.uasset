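; BP_HitBox_First is a hit box actor that shrinks each time another actor stops overlapping it.
; BeginPlay caches five percent of the starting scale in Our5, and each end overlap subtracts that fixed step, so shrinking is linear with no lower clamp.
; Begin overlap only forwards to the parent class, and Tick is disabled.
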(event EventBeginPlay
  (Variables|Default|SetOur%205%25 (* (Transformation|GetActorScale3D) 0.05)))

(event Collision|EventActorBeginOverlap
  (params (OtherActor :type Actor%20Object%20Reference))
  (|CallParentFunction OtherActor))

(event EventTick
  (params (DeltaSeconds :type Float%20%28single-precision%29))
  (|CallParentFunction DeltaSeconds) ; This node is disabled and will not be called.\nDrag off pins to build functionality.
)

(event Collision|EventActorEndOverlap
  (params (OtherActor :type Actor%20Object%20Reference))
  (Transformation|SetActorScale3D (- (Transformation|GetActorScale3D) (Variables|Default|GetOur%205%25))))

(fn ConstructionScript
  (|CallParentFunction))