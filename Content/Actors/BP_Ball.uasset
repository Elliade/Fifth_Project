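; BP_Ball is an actor that moves in a straight line and bounces off blocking surfaces.
; Tick offsets it along Direction by Velocity scaled by delta time, using a swept move to detect hits rather than physics simulation.
; Each blocking hit reflects Direction about the hit normal, cuts speed by a fixed percentage clamped at MinVelocity, and prints the new speed for debugging.
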(event EventBeginPlay)

(event Collision|EventActorBeginOverlap
  (params (OtherActor :type Actor%20Object%20Reference)))

(event EventTick
  (params (DeltaSeconds :type Float%20%28single-precision%29))
  (bind _sweephitresult (Transformation|AddActorWorldOffset (* (* (Variables|Default|GetDirection) (Variables|Default|GetVelocity)) DeltaSeconds) true))
  (if (.bBlockingHit (Collision|BreakHitResult _sweephitresult))
    ;[1 1 1] Проверка условия скорости
    (if (<= (- (Variables|Default|GetVelocity) (* (Variables|Default|GetVelocity) 0.1)) (Variables|Default|GetMinVelocity))
      (bind _output_get (Variables|Default|SetVelocity (Variables|Default|GetMinVelocity)))
      (else
        (Variables|Default|SetVelocity (- (Variables|Default|GetVelocity) (* (Variables|Default|GetVelocity) 0.1)))))
    (Variables|Default|SetDirection (Math|Vector|GetReflectionVector (Variables|Default|GetDirection) (.Normal (Collision|BreakHitResult _sweephitresult))))
    ;[1 1 1] Вывод скорости
    (Development|PrintString (Utilities|String|ToString(Float) _output_get))))

(fn ConstructionScript)