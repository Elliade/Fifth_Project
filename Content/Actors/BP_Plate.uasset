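; BP_Plate is a player-controlled paddle that slides along the X axis and spawns a ball.
; On BeginPlay, SpawnBall creates a BP_Ball at the Capsule's location, stores it and binds an event to its OnDead dispatcher.
; The Move input axis shifts the plate by a fixed, swept world offset per call, based only on the input's sign, without delta-time scaling.
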(event EventBeginPlay
  ;[1 1 1] Спавним шар
  (CallFunction|SpawnBall))

(event Collision|EventActorBeginOverlap
  (params (OtherActor :type Actor%20Object%20Reference)))

(event EventTick
  (params (DeltaSeconds :type Float%20%28single-precision%29)))

(event Input|AxisEvents|InputAxisMove
  (params (AxisValue :type Float%20%28single-precision%29))
  ;[1 1 1] Ось Х минус
  (if (< AxisValue 0.0)
    (Transformation|AddActorWorldOffset "-50.000000,0.000000,0.000000" true)))

(event Input|AxisEvents|InputAxisMove
  (params (AxisValue :type Float%20%28single-precision%29))
  ;[1 1 1] Ось Х плюс
  (if (> AxisValue 0.0)
    (Transformation|AddActorWorldOffset "50.000000,0.000000,0.000000" true)))

(fn ConstructionScript)

(fn SpawnBall
  (bind _returnvalue (Game|SpawnActorfromClass "/Game/Actors/BP_Ball.BP_Ball_C" (Math|Transform|MakeTransform (Transformation|GetWorldLocation (Variables|Default|GetCapsule)) "0, 0, 0" "1.000000,1.000000,1.000000") "AlwaysSpawn" "MultiplyWithRoot" 0 0))
  (bind _output_get (Variables|Default|SetNewVar _returnvalue))
  (EventDispatchers|BindEventtoOnDead _output_get (EventDispatchers|CreateEvent :!event SpawnBall)))